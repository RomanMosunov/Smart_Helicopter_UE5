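; Player-controlled helicopter pawn that fakes flight without physics, using Enhanced Input and movement input.
; Pitch and roll move it and tilt the mesh within limits, while other actions yaw the actor and change altitude.
; Releasing input plays a timeline that adds inertia scaled by hold time and blends the tilt between level and its release rotation; new input stops it.
; A looping timer turns the rotor, and Tick prints actor rotation for debugging.
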(event Custom|StopTL
  (bind _newtrack_0 (Timeline|InertiaTL Stop)
    (:Update
      (CallFunction|PitchInertia _newtrack_0)
      (CallFunction|RollInertia _newtrack_0)
      (CallFunction|Alignment _newtrack_0)
      (CallFunction|LiftInertia _newtrack_0))))

(event Input|EnhancedActionEvents|EnhancedInputActionIA_Pitch
  (params (ActionValue :type Float%20%28double-precision%29) (ElapsedSeconds :type Float%20%28double-precision%29) (TriggeredSeconds :type Float%20%28double-precision%29) (InputAction :type Input%20Action%20Object%20Reference :default "/Game/Input/IA_Pitch.IA_Pitch"))
  (:Completed
    (CallFunction|SetValues TriggeredSeconds (stale Input|EnhancedActionEvents|EnhancedInputActionIA_Roll TriggeredSeconds) (stale Input|EnhancedActionEvents|EnhancedInputActionIA_UpDown TriggeredSeconds))
    (bind _newtrack_0 (Timeline|InertiaTL PlayFromStart)
      (:Update
        (CallFunction|PitchInertia _newtrack_0)
        (CallFunction|RollInertia _newtrack_0)
        (CallFunction|Alignment _newtrack_0)
        (CallFunction|LiftInertia _newtrack_0)))))

(event Input|EnhancedActionEvents|EnhancedInputActionIA_Roll
  (params (ActionValue :type Float%20%28double-precision%29) (ElapsedSeconds :type Float%20%28double-precision%29) (TriggeredSeconds :type Float%20%28double-precision%29) (InputAction :type Input%20Action%20Object%20Reference :default "/Game/Input/IA_Roll.IA_Roll"))
  (:Completed
    (CallFunction|SetValues (stale Input|EnhancedActionEvents|EnhancedInputActionIA_Pitch TriggeredSeconds) TriggeredSeconds (stale Input|EnhancedActionEvents|EnhancedInputActionIA_UpDown TriggeredSeconds))
    (bind _newtrack_0 (Timeline|InertiaTL PlayFromStart)
      (:Update
        (CallFunction|PitchInertia _newtrack_0)
        (CallFunction|RollInertia _newtrack_0)
        (CallFunction|Alignment _newtrack_0)
        (CallFunction|LiftInertia _newtrack_0)))))

(event Input|EnhancedActionEvents|EnhancedInputActionIA_Rotate
  (params (ActionValue :type Float%20%28double-precision%29) (ElapsedSeconds :type Float%20%28double-precision%29) (TriggeredSeconds :type Float%20%28double-precision%29) (InputAction :type Input%20Action%20Object%20Reference :default "/Game/Input/IA_Rotate.IA_Rotate"))
  (:Completed
    (CallFunction|SetValues (stale Input|EnhancedActionEvents|EnhancedInputActionIA_Pitch TriggeredSeconds) (stale Input|EnhancedActionEvents|EnhancedInputActionIA_Roll TriggeredSeconds) (stale Input|EnhancedActionEvents|EnhancedInputActionIA_UpDown TriggeredSeconds))
    (bind _newtrack_0 (Timeline|InertiaTL PlayFromStart)
      (:Update
        (CallFunction|PitchInertia _newtrack_0)
        (CallFunction|RollInertia _newtrack_0)
        (CallFunction|Alignment _newtrack_0)
        (CallFunction|LiftInertia _newtrack_0)))))

(event Input|EnhancedActionEvents|EnhancedInputActionIA_UpDown
  (params (ActionValue :type Float%20%28double-precision%29) (ElapsedSeconds :type Float%20%28double-precision%29) (TriggeredSeconds :type Float%20%28double-precision%29) (InputAction :type Input%20Action%20Object%20Reference :default "/Game/Input/IA_UpDown.IA_UpDown"))
  (:Completed
    (CallFunction|SetValues (stale Input|EnhancedActionEvents|EnhancedInputActionIA_Pitch TriggeredSeconds) (stale Input|EnhancedActionEvents|EnhancedInputActionIA_Roll TriggeredSeconds) TriggeredSeconds)
    (bind _newtrack_0 (Timeline|InertiaTL PlayFromStart)
      (:Update
        (CallFunction|PitchInertia _newtrack_0)
        (CallFunction|RollInertia _newtrack_0)
        (CallFunction|Alignment _newtrack_0)
        (CallFunction|LiftInertia _newtrack_0)))))

(event Input|EnhancedActionEvents|EnhancedInputActionIA_Pitch
  (params (ActionValue :type Float%20%28double-precision%29) (ElapsedSeconds :type Float%20%28double-precision%29) (TriggeredSeconds :type Float%20%28double-precision%29) (InputAction :type Input%20Action%20Object%20Reference :default "/Game/Input/IA_Pitch.IA_Pitch"))
  (bind _output_get (Variables|Default|SetPitchDir ActionValue))
  (Variables|Default|SetRollDir 0.0)
  (CallFunction|Pitch _output_get)
  (CallFunction|StopTL))

(event Input|EnhancedActionEvents|EnhancedInputActionIA_Roll
  (params (ActionValue :type Float%20%28double-precision%29) (ElapsedSeconds :type Float%20%28double-precision%29) (TriggeredSeconds :type Float%20%28double-precision%29) (InputAction :type Input%20Action%20Object%20Reference :default "/Game/Input/IA_Roll.IA_Roll"))
  (bind _output_get (Variables|Default|SetRollDir ActionValue))
  (Variables|Default|SetPitchDir 0.0)
  (CallFunction|Roll _output_get)
  (CallFunction|StopTL))

(event Input|EnhancedActionEvents|EnhancedInputActionIA_Rotate
  (params (ActionValue :type Float%20%28double-precision%29) (ElapsedSeconds :type Float%20%28double-precision%29) (TriggeredSeconds :type Float%20%28double-precision%29) (InputAction :type Input%20Action%20Object%20Reference :default "/Game/Input/IA_Rotate.IA_Rotate"))
  (Class|Actor|AddActorWorldRotation (Math|Rotator|MakeRotator 0.0 0.0 ActionValue))
  (CallFunction|StopTL))

(event Input|EnhancedActionEvents|EnhancedInputActionIA_UpDown
  (params (ActionValue :type Float%20%28double-precision%29) (ElapsedSeconds :type Float%20%28double-precision%29) (TriggeredSeconds :type Float%20%28double-precision%29) (InputAction :type Input%20Action%20Object%20Reference :default "/Game/Input/IA_UpDown.IA_UpDown"))
  (Pawn|Input|AddMovementInput (Math|Vector|GetUpVector "0, 0, 0") ActionValue false)
  (CallFunction|StopTL))

(event EventBeginPlay
  (bind _returnvalue (Game|GetPlayerController 0))
  (bind _returnvalue_2 (PlayerController|LocalPlayerSubsystems|GetEnhancedInputLocalPlayerSubsystem _returnvalue))
  (Utilities|Time|SetTimerbyFunctionName 0 "Rotor" 0.001 true)
  (Utilities|IsValid _returnvalue
    (:Is%20Valid
      (Utilities|IsValid _returnvalue_2
        (:Is%20Valid
          (Input|AddMappingContext _returnvalue_2 "/Game/Input/IMC_Default.IMC_Default" 0 "(bIgnoreAllPressedKeysUntilRelease=True,bForceImmediately=False,bNotifyUserSettings=False)")
          (Input|SetInputModeGameOnly _returnvalue false))))))

(event EventTick
  (params (DeltaSeconds :type Float%20%28single-precision%29))
  (Development|PrintString (Utilities|String|ToString(Rotator) (Transformation|GetActorRotation))))

(fn ConstructionScript)

(fn Pitch
  (params (ActionValue :type Float%20%28double-precision%29))
  (Pawn|Input|AddMovementInput (Transformation|GetActorForwardVector) ActionValue false)
  (if (Math|Float|InRange(Float) (.pitch (Variables|/Script/Engine.SceneComponent|GetRelativeRotation (Variables|Default|GetCopterMesh))) -4e+01 4e+01 false false)
    (Transformation|AddRelativeRotation (Variables|Default|GetCopterMesh) (Math|Rotator|MakeRotator 0.0 (* ActionValue -1.0) 0.0) false false)))

(fn Roll
  (params (ActionValue :type Float%20%28double-precision%29))
  (Pawn|Input|AddMovementInput (Transformation|GetActorRightVector) ActionValue false)
  (if (Math|Float|InRange(Float) (.roll (Variables|/Script/Engine.SceneComponent|GetRelativeRotation (Variables|Default|GetCopterMesh))) -4e+01 4e+01 false false)
    (Transformation|AddRelativeRotation (Variables|Default|GetCopterMesh) (Math|Rotator|MakeRotator ActionValue 0.0 0.0) false false)))

(fn SetValues
  (params (PitchSec :type Float%20%28double-precision%29) (RollSec :type Float%20%28double-precision%29) (MoveUpSec :type Float%20%28double-precision%29))
  (Variables|Default|SetRotation (Variables|/Script/Engine.SceneComponent|GetRelativeRotation (Variables|Default|GetCopterMesh)))
  (Variables|Default|SetPitchSec PitchSec)
  (Variables|Default|SetRollSec RollSec)
  (Variables|Default|SetMoveUpSec MoveUpSec))

(fn Alignment
  (params (Alpha :type Float%20%28double-precision%29))
  (Transformation|SetRelativeRotation (Variables|Default|GetCopterMesh) (Math|Rotator|Lerp(Rotator) (Math|Rotator|MakeRotator 0.0 0.0 (.yaw (Variables|/Script/Engine.SceneComponent|GetRelativeRotation (Variables|Default|GetCopterMesh)))) (Variables|Default|GetRotation) Alpha) false false))

(fn PitchInertia
  (params (Alpha :type Float%20%28double-precision%29))
  (Pawn|Input|AddMovementInput (Transformation|GetActorForwardVector) (* Alpha (Variables|Default|GetPitchDir) (Variables|Default|GetPitchSec)) false))

(fn RollInertia
  (params (Alpha :type Float%20%28double-precision%29))
  (Pawn|Input|AddMovementInput (Transformation|GetActorRightVector) (* Alpha (Variables|Default|GetRollDir) (Variables|Default|GetRollSec)) false))

(fn LiftInertia
  (params (Alpha :type Float%20%28double-precision%29))
  (Pawn|Input|AddMovementInput (Math|Vector|GetUpVector "0, 0, 0") (* Alpha (Variables|Default|GetMoveUpSec) (Math|Float|Clamp(Float) (.z (Transformation|GetVelocity)) -1.0)) false))

(fn Rotor
  (Transformation|AddRelativeRotation (Variables|Default|GetCube) (Math|Rotator|MakeRotator 0.0 0.0 (Math|Trig|Sin(Degrees) (Variables|Default|GetRotorSpeed))) false false))