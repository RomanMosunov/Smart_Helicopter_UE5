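; Physics-driven, player-controlled helicopter that flies via Enhanced Input, using a thruster for lift and torques for yaw, pitch and roll.
; Lift scales with mass and compensates for tilt, with center of mass aligned to the thruster in local X/Y at BeginPlay.
; Releasing pitch or roll starts a timeline that levels the body while keeping yaw; flight input stops it.
; A looping timer spins the rotor.
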(event Custom|Alignment
  ;[1 1 1] Alignment
  (Variables|Default|SetRot (Transformation|GetWorldRotation (Variables|Default|GetCopterMesh)))
  (bind _newtrack_0 (Timeline|Timeline PlayFromStart)
    (:Update
      (Transformation|SetWorldRotation (Variables|Default|GetCopterMesh) (Math|Rotator|Lerp(Rotator) (Variables|Default|GetRot) (Math|Rotator|MakeRotator 0.0 0.0 (.yaw (Variables|Default|GetRot))) _newtrack_0) false false))))

(event Custom|StopTL
  ;[1 1 1] Alignment
  (bind _newtrack_0 (Timeline|Timeline Stop)
    (:Update
      (Transformation|SetWorldRotation (Variables|Default|GetCopterMesh) (Math|Rotator|Lerp(Rotator) (Variables|Default|GetRot) (Math|Rotator|MakeRotator 0.0 0.0 (.yaw (Variables|Default|GetRot))) _newtrack_0) false false))))

(event Input|EnhancedActionEvents|EnhancedInputActionIA_Pitch
  (params (ActionValue :type Float%20%28double-precision%29) (ElapsedSeconds :type Float%20%28double-precision%29) (TriggeredSeconds :type Float%20%28double-precision%29) (InputAction :type Input%20Action%20Object%20Reference :default "/Game/Input/IA_Pitch.IA_Pitch"))
  ;[1 1 1] Pitch
  (:Triggered
    (CallFunction|StopTL)
    (Class|PrimitiveComponent|AddTorqueinDegrees (Variables|Default|GetCopterMesh) (* (Transformation|GetActorRightVector) (Math|Float|Clamp(Float) (+ (* ActionValue 3e+01) (.pitch (Transformation|GetWorldRotation (Variables|Default|GetCopterMesh)))) -2e+01 2e+01) 5.0) "None" true))
  (:Completed
    (CallFunction|Alignment)))

(event Input|EnhancedActionEvents|EnhancedInputActionIA_Roll
  (params (ActionValue :type Float%20%28double-precision%29) (ElapsedSeconds :type Float%20%28double-precision%29) (TriggeredSeconds :type Float%20%28double-precision%29) (InputAction :type Input%20Action%20Object%20Reference :default "/Game/Input/IA_Roll.IA_Roll"))
  ;[1 1 1] Roll
  (:Triggered
    (CallFunction|StopTL)
    (Class|PrimitiveComponent|AddTorqueinDegrees (Variables|Default|GetCopterMesh) (* (Transformation|GetActorForwardVector) (Math|Float|Clamp(Float) (+ (* ActionValue -45.0) (.roll (Transformation|GetWorldRotation (Variables|Default|GetCopterMesh)))) -2e+01 2e+01) 5.0) "None" true))
  (:Completed
    (CallFunction|Alignment)))

(event Input|EnhancedActionEvents|EnhancedInputActionIA_Rotate
  (params (ActionValue :type Float%20%28double-precision%29) (ElapsedSeconds :type Float%20%28double-precision%29) (TriggeredSeconds :type Float%20%28double-precision%29) (InputAction :type Input%20Action%20Object%20Reference :default "/Game/Input/IA_Rotate.IA_Rotate"))
  ;[1 1 1] Rotation
  (CallFunction|StopTL)
  (Class|PrimitiveComponent|AddTorqueinDegrees (Variables|Default|GetCopterMesh) (* ActionValue (Transformation|GetActorUpVector) (Variables|Default|GetRotationSpeed)) "None" true))

(event Input|EnhancedActionEvents|EnhancedInputActionIA_UpDown
  (params (ActionValue :type Float%20%28double-precision%29) (ElapsedSeconds :type Float%20%28double-precision%29) (TriggeredSeconds :type Float%20%28double-precision%29) (InputAction :type Input%20Action%20Object%20Reference :default "/Game/Input/IA_UpDown.IA_UpDown"))
  ;[1 1 1] MoveUpDown
  (CallFunction|StopTL)
  (Variables|/Script/Engine.PhysicsThrusterComponent|SetThrustStrength (Variables|Default|GetPhysicsThruster) (* (/ (+ (* ActionValue (Variables|Default|GetLiftStrenght)) 1e+03) (.z (Transformation|GetActorUpVector))) (Physics|GetMass (Variables|Default|GetCopterMesh)))))

(event EventBeginPlay
  (bind _returnvalue (Game|GetPlayerController 0))
  (bind _physicsthruster (Variables|Default|GetPhysicsThruster))
  (bind _coptermesh (Variables|Default|GetCopterMesh))
  (bind _coptermesh_2 (Variables|Default|GetCopterMesh))
  (bind _returnvalue_2 (Transformation|GetWorldLocation _physicsthruster))
  (bind _returnvalue_3 (Physics|GetCenterOfMass _coptermesh "None"))
  (bind _returnvalue_4 (Transformation|GetWorldRotation _coptermesh_2))
  (bind _returnvalue_5 (PlayerController|LocalPlayerSubsystems|GetEnhancedInputLocalPlayerSubsystem _returnvalue))
  (bind _returnvalue_6 (Class|KismetMathLibrary|NegateRotator _returnvalue_4))
  (bind _returnvalue_7 (- _returnvalue_2 _returnvalue_3))
  (bind _returnvalue_8 (Math|Vector|RotateVector _returnvalue_7 _returnvalue_6))
  ;[1 1 1] SetCenterOfMass
  (Class|PrimitiveComponent|SetCenterOfMass (Variables|Default|GetCopterMesh) (Math|Vector|MakeVector (.x _returnvalue_8) (.y _returnvalue_8) 0.0) "None")
  (Utilities|Time|SetTimerbyFunctionName 0 "Rotor" 0.001 true)
  (Utilities|IsValid _returnvalue
    (:Is%20Valid
      (Utilities|IsValid _returnvalue_5
        (:Is%20Valid
          (Input|AddMappingContext _returnvalue_5 "/Game/Input/IMC_Default.IMC_Default" 0 "(bIgnoreAllPressedKeysUntilRelease=True,bForceImmediately=False,bNotifyUserSettings=False)")
          (Input|SetInputModeGameOnly _returnvalue false))))))

(event EventTick
  (params (DeltaSeconds :type Float%20%28single-precision%29))
  (Development|PrintString (Utilities|String|ToString(Rotator) (Transformation|GetWorldRotation (Variables|Default|GetCopterMesh)))))

(event Input|KeyboardEvents|1
  (params (Key :type Key%20Structure))
  (:Pressed
    (Game|OpenLevel(byName) "Map_2_Mobile")))

(fn ConstructionScript)

(fn Rotor
  (Transformation|AddRelativeRotation (Variables|Default|GetCube) (Math|Rotator|MakeRotator 0.0 0.0 (Math|Trig|Sin(Degrees) (Variables|Default|GetRotorSpd))) false false))